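; VS_player_controler is a player-controller Blueprint that handles input for player character 0 and caches the game state as Mygamestate on BeginPlay.
; MoveRight moves the character along the fixed world Y axis, and Jump triggers a jump and clears the Jumping flag.
; Sub Attack and Dash only print debug strings.
; The attack events are empty, and the montage attack and launch logic is left unwired.
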(event `self.ReceiveBeginPlay`
  ;[1 1 1] Event begin play
  (bind _asmygamestate (cast `/Game/Blueprints/Mygamestate` (`GameplayStatics.GetGameState`)))
  (set `self.Mygamestate` _asmygamestate))

(event `InputAction|Main Attack`
  (params (Key :type "Key Structure" :default "AnyKey")))

(event `InputAxis|MoveRight`
  (params (AxisValue :type "Float (single-precision)"))
  (bind _returnvalue (`GameplayStatics.GetPlayerCharacter` 0))
  ;[1 1 1] Movement
  (`/Engine/EditorBlueprintResources/StandardMacros.IsValid` _returnvalue
    (:`Is Valid`
      (`Pawn.AddMovementInput` _returnvalue (0.0 1.0 0.0) AxisValue false))))

(event `Sword Attack`)

(event `Attack end`)

(event `InputAction|Jump`
  (params (Key :type "Key Structure" :default "AnyKey"))
  (bind _returnvalue (`GameplayStatics.GetPlayerCharacter` 0))
  ;[1 1 1] action
  (:`Pressed`
    (`/Engine/EditorBlueprintResources/StandardMacros.IsValid` _returnvalue
      (:`Is Valid`
        (`Character.Jump` _returnvalue)
        (set `self.Jumping` false)))))

(event `InputAction|Sub Attack`
  (params (Key :type "Key Structure" :default "AnyKey")))

(event `attack 2`)

(event `attack 2 end`)

(event `InputAction|Sub Attack`
  (params (Key :type "Key Structure" :default "AnyKey"))
  ;[1 1 1] Comment
  (:`Pressed`
    (`KismetSystemLibrary.PrintString` "using sub attack")))

(event `InputAction|Dash`
  (params (Key :type "Key Structure" :default "AnyKey"))
  ;[1 1 1] Comment
  (:`Pressed`
    (`KismetSystemLibrary.PrintString` "using dash ")))

(event `InputAction|Sub Attack`
  (params (Key :type "Key Structure" :default "AnyKey")))

(fn `UserConstructionScript`)
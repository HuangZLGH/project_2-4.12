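; Test controller Blueprint, apparently a prototype for side-on character movement and actions.
; MoveRight input moves player character 1 along the world Y axis, while Jump acts on player character 0 and clears a Jumping flag.
; Sword attack events are empty stubs.
; Montage-timed attacks, a capsule-relative dash launch and debug prints are left unconnected, so they never run.
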(event `InputAction|Main Attack`
  (params (Key :type "Key Structure" :default "AnyKey")))

(event `Sword Attack`)

(event `InputAxis|MoveRight` :consume false :overrideparent false
  (params (AxisValue :type "Float (single-precision)"))
  ;[1 1 1] Movement
  (`Pawn.AddMovementInput` (`GameplayStatics.GetPlayerCharacter` 1) (0.0 -1.0 0.0) AxisValue false))

(event `Attack end`)

(event `InputAction|Sub Attack`
  (params (Key :type "Key Structure" :default "AnyKey")))

(event `attack 2`)

(event `attack 2 end`)

(event `InputAction|Jump`
  (params (Key :type "Key Structure" :default "AnyKey"))
  ;[1 1 1] action
  (:`Pressed`
    (`Character.Jump` (`GameplayStatics.GetPlayerCharacter` 0))
    (set `self.Jumping` false)))

(event `InputAction|Sub Attack`
  (params (Key :type "Key Structure" :default "AnyKey")))

(event `InputAction|Sub Attack`
  (params (Key :type "Key Structure" :default "AnyKey"))
  ;[1 1 1] Comment
)

(event `InputAction|Dash`
  (params (Key :type "Key Structure" :default "AnyKey"))
  ;[1 1 1] Comment
)

(fn `UserConstructionScript`)
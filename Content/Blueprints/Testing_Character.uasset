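; Test character that animates a four-segment tail toggled by a TailOn flag read from the game state each Tick.
; While on, Curve1 sets the Y offsets of Mesh1-4 at increasing multiples to spread them out as a chain.
; While off, Curve2 drives the offsets and the meshes hide when they reach zero.
; It also clears Jumping on landing and spawns and possesses a second local player on key 3.
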(event `self.ReceiveActorBeginOverlap`
  (params (OtherActor :type "Actor Object Reference")))

(event `Key|Three`
  (params (Key :type "Key Structure" :default "AnyKey"))
  (:`Pressed`
    (bind _returnvalue (`GameplayStatics.CreatePlayer` 1))
    (`Controller.Possess` _returnvalue (`GameplayStatics.GetPlayerCharacter` 1))))

(event `self.OnLanded`
  (params (Hit :type "HitResult Structure (by ref)"))
  ;[1 1 1] event on laned
  (set `self.Jumping` false))

(event `self.ReceiveTick`
  (params (DeltaSeconds :type "Float (single-precision)"))
  (bind _returnvalue (`KismetMathLibrary.MakeVector` 0.0 (`CurveFloat.GetFloatValue` (`self.curve_2`) (`self.time2`))))
  (`|ExecutionSequence`
    (:`then_0`
      (bind _asmygamestate (cast `/Game/Blueprints/Mygamestate` (`GameplayStatics.GetGameState`)))
      (set `self.tail on?` (`/Game/Blueprints/Mygamestate.tail_on` _asmygamestate)))
    (:`then_1`
      (if (`self.tail on?`)
        (set `self.time2` 0.0)
        (set `self.time` (+ (`self.time`) DeltaSeconds))
        (else
          (set `self.time` 0.0)
          (set `self.time2` (+ (`self.time2`) DeltaSeconds))
          (`|ExecutionSequence`
            (:`then_0`
              (`/Engine/EditorBlueprintResources/StandardMacros.DoOnce` false
                (:`Completed`
                  (`SceneComponent.SetVisibility` (`self.Mesh1`) false false)
                  (`SceneComponent.SetVisibility` (`self.Mesh2`) false false)
                  (`SceneComponent.SetVisibility` (`self.Mesh3`) false false)
                  (`SceneComponent.SetVisibility` (`self.Mesh4`) false false))))
            (:`then_1`
              _))))
      (if (`self.tail on?`)
        (`SceneComponent.SetVisibility` (`self.Mesh1`) true false)
        (`SceneComponent.SetVisibility` (`self.Mesh2`) true false)
        (`SceneComponent.SetVisibility` (`self.Mesh3`) true false)
        (`SceneComponent.SetVisibility` (`self.Mesh4`) true false)
        (`|ExecutionSequence`
          (:`then_0`
            (`SceneComponent.K2_SetRelativeLocation` (`self.Mesh1`) (`KismetMathLibrary.MakeVector` 0.0 (`CurveFloat.GetFloatValue` (`self.curve_1`) (`self.time`))) false false))
          (:`then_1`
            (`SceneComponent.K2_SetRelativeLocation` (`self.Mesh2`) (`KismetMathLibrary.MakeVector` 0.0 (* (`CurveFloat.GetFloatValue` (`self.curve_1`) (`self.time`)) 2.0)) false false))
          (:`then_2`
            (`SceneComponent.K2_SetRelativeLocation` (`self.Mesh3`) (`KismetMathLibrary.MakeVector` 0.0 (* (`CurveFloat.GetFloatValue` (`self.curve_1`) (`self.time`)) 3.0)) false false))
          (:`then_3`
            (`SceneComponent.K2_SetRelativeLocation` (`self.Mesh4`) (`KismetMathLibrary.MakeVector` 0.0 (* (`CurveFloat.GetFloatValue` (`self.curve_1`) (`self.time`)) 4.0)) false false)))
        (else
          (`|ExecutionSequence`
            (:`then_0`
              (`SceneComponent.K2_SetRelativeLocation` (`self.Mesh1`) _returnvalue false false)
              (if (== _returnvalue (0.0 0.0 0.0) :`ErrorTolerance` 0.0)
                (`SceneComponent.SetVisibility` (`self.Mesh1`) (`self.tail on?`) false)
                (`SceneComponent.SetVisibility` (`self.Mesh2`) (`self.tail on?`) false)
                (`SceneComponent.SetVisibility` (`self.Mesh3`) (`self.tail on?`) false)
                (`SceneComponent.SetVisibility` (`self.Mesh4`) (`self.tail on?`) false)
                (`self.reset`)))
            (:`then_1`
              (`SceneComponent.K2_SetRelativeLocation` (`self.Mesh2`) (`KismetMathLibrary.MakeVector` 0.0 (* (`CurveFloat.GetFloatValue` (`self.curve_2`) (`self.time2`)) 2.0)) false false))
            (:`then_2`
              (`SceneComponent.K2_SetRelativeLocation` (`self.Mesh3`) (`KismetMathLibrary.MakeVector` 0.0 (* (`CurveFloat.GetFloatValue` (`self.curve_2`) (`self.time2`)) 3.0)) false false))
            (:`then_3`
              (`SceneComponent.K2_SetRelativeLocation` (`self.Mesh4`) (`KismetMathLibrary.MakeVector` 0.0 (* (`CurveFloat.GetFloatValue` (`self.curve_2`) (`self.time2`)) 4.0)) false false))))))))

(event `reset`)

(fn `UserConstructionScript`)